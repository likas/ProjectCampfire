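; VR player character that lets the player grab and drop objects with either motion controller.
; Each hand's primary grip input runs a shared PerformGrip on press and ReleaseGrip on release.
; Gripping sphere-overlaps WorldDynamic actors at the controller and grips the first at its current transform, drawing a debug sphere larger than the query.
; Releasing drops every grip on that controller with physics simulation enabled.
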(event Custom|ReleaseGrip
  (params (Controller :type Grip%20Motion%20Controller%20Component%20Object%20Reference))
  (bind _griparray (Class|GripMotionControllerComponent|GetAllGrips Controller))
  (for _array_element _griparray
    (Class|GripMotionControllerComponent|DropGrip Controller _array_element true "0, 0, 0" "0, 0, 0")))

(event Custom|PerformGrip
  (params (Controller :type Grip%20Motion%20Controller%20Component%20Object%20Reference))
  (bind _returnvalue (Transformation|GetWorldLocation Controller))
  (Rendering|Debug|DrawDebugSphere _returnvalue 1e+01 12 "(R=1.000000,G=1.000000,B=1.000000,A=1.000000)" 1.0 1.0)
  (bind (_outactors _returnvalue_2) (Collision|SphereOverlapActors _returnvalue 5.0 (Utilities|Array|MakeArray "ObjectTypeQuery2") 0 (Utilities|Array|MakeArray self)))
  (if _returnvalue_2
    (Class|GripMotionControllerComponent|GripActor Controller (Utilities|Array|Get(acopy) _outactors) (Transformation|GetActorTransform (Utilities|Array|Get(acopy) _outactors)) false "None" "None" "InteractiveCollisionWithPhysics" "NotWhenCollidingOrDoubleGripping" "ForceClientSideMovement" 1.5e+03 2e+02 false)))

(event EventBeginPlay)

(event Collision|EventActorBeginOverlap
  (params (OtherActor :type Actor%20Object%20Reference)))

(event EventTick
  (params (DeltaSeconds :type Float%20%28single-precision%29)))

(event Input|ActionEvents|InputActionPrimaryGripRight
  (params (Key :type Key%20Structure :default "None"))
  (bind _rightmotioncontroller (Variables|Default|GetRightMotionController))
  (:Pressed
    (CallFunction|PerformGrip _rightmotioncontroller))
  (:Released
    (CallFunction|ReleaseGrip _rightmotioncontroller)))

(event Input|ActionEvents|InputActionPrimaryGripLeft
  (params (Key :type Key%20Structure :default "None"))
  (bind _leftmotioncontroller (Variables|Default|GetLeftMotionController))
  (:Pressed
    (CallFunction|PerformGrip _leftmotioncontroller))
  (:Released
    (CallFunction|ReleaseGrip _leftmotioncontroller)))

(fn ConstructionScript)